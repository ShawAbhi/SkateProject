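; Player-following grid of instanced meshes for the trail system, conforming to ground height around the character.
; The construction script lays out a square grid from CellRange and CellSize.
; Tick writes the player location to MPC_CustomTrails and snaps the actor to the player's truncated cell position.
; When that snapped position changes, vertical line traces move each instance's height to just above the hit surface, keeping rotation and scale.
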(event `self.ReceiveTick`
  (params (DeltaSeconds :type "Float (single-precision)"))
  (bind _instancedstaticmesh (`self.InstancedStaticMesh`))
  (bind _cellsize (`self.CellSize`))
  (bind _returnvalue (`self.K2_GetActorLocation` (`GameplayStatics.GetPlayerCharacter` 0)))
  (bind (_returnvalue_x _returnvalue_y _returnvalue_z) (`KismetMathLibrary.BreakVector` (/ _returnvalue (`self.CellSize`))))
  (`KismetMaterialLibrary.SetVectorParameterValue` "/Game/TrailSystem/Blueprints/MPC_CustomTrails.MPC_CustomTrails" "PlayerLocation" (`KismetMathLibrary.Conv_VectorToLinearColor` _returnvalue))
  (`self.K2_SetActorLocation` (`KismetMathLibrary.MakeVector` (* (`KismetMathLibrary.FTrunc` _returnvalue_x) _cellsize) (* (`KismetMathLibrary.FTrunc` _returnvalue_y) _cellsize) (* (`KismetMathLibrary.FTrunc` _returnvalue_z) (`self.CellSize`))) false true)
  (if (!= (`self.CacheActorLocation`) (`self.K2_GetActorLocation`))
    (set `self.CacheActorLocation` (`self.K2_GetActorLocation`))
    (for _index (range 1 (+ (`InstancedStaticMeshComponent.GetInstanceCount` (`self.InstancedStaticMesh`)) 1))
      (bind _returnvalue_2 (- _index 1))
      (bind _outinstancetransform (`InstancedStaticMeshComponent.GetInstanceTransform` (`self.InstancedStaticMesh`) _returnvalue_2 true))
      (bind (_outhit _returnvalue_3) (`KismetSystemLibrary.LineTraceSingle` (+ (.location _outinstancetransform) (* (`KismetMathLibrary.Vector_Up`) 1000.0)) (+ (.location _outinstancetransform) (* (`KismetMathLibrary.Vector_Down`) 1000.0)) "TraceTypeQuery3"))
      (if _returnvalue_3
        (bind _outinstancetransform_2 (`InstancedStaticMeshComponent.GetInstanceTransform` _instancedstaticmesh _returnvalue_2 true))
        (bind (_bblockinghit _binitialoverlap _time _distance _location _impactpoint _normal) (`GameplayStatics.BreakHitResult` _outhit))
        (`InstancedStaticMeshComponent.UpdateInstanceTransform` _instancedstaticmesh _returnvalue_2 (`KismetMathLibrary.MakeTransform` (`KismetMathLibrary.MakeVector` (.x (.location _outinstancetransform_2)) (.y (.location _outinstancetransform_2)) (.z (+ _impactpoint (* _normal 10.0)))) (.rotation _outinstancetransform_2) (.scale _outinstancetransform_2)) true true true)))))

(fn `UserConstructionScript`
  (bind _cellrange (`self.CellRange`))
  (bind _cellrange_2 (`self.CellRange`))
  (for _index (range (* _cellrange -1) (+ _cellrange 1))
    (for _index_2 (range (* _cellrange_2 -1) (+ _cellrange_2 1))
      (`InstancedStaticMeshComponent.AddInstance` (`self.InstancedStaticMesh`) (`KismetMathLibrary.MakeTransform` (`KismetMathLibrary.MakeVector` (* _index (`self.CellSize`)) (* _index_2 (`self.CellSize`)))) false))))