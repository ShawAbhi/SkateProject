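; Scene component that paints movement trails into the RT_Trails render target, which it clears on BeginPlay.
; Each tick it writes current and previous locations of the player and the component, plus the component's remapped yaw, to the MPC_CustomTrails parameter collection.
; It then draws M_Rect into the render target and caches the current values as the next frame's previous ones.
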(event `self.ReceiveBeginPlay`
  (bind (_returnvalue_roll _returnvalue_pitch _returnvalue_yaw) (`KismetMathLibrary.BreakRotator` (`self.K2_GetComponentRotation`)))
  (set `self.CachedLocation` (`self.K2_GetComponentLocation`))
  (set `self.CachedYaw` (+ (/ (+ _returnvalue_yaw 180.0) 180.0) 0.5))
  (`KismetRenderingLibrary.ClearRenderTarget2D` "/Game/TrailSystem/Blueprints/RT_Trails.RT_Trails" (struct)))

(event `self.ReceiveTick`
  (params (DeltaSeconds :type "Float (single-precision)"))
  (`self.PaintTrails`))

(fn `PaintTrails`
  (bind (_returnvalue_roll _returnvalue_pitch _returnvalue_yaw) (`KismetMathLibrary.BreakRotator` (`self.K2_GetComponentRotation`)))
  (`|ExecutionSequence`
    (:`then_0`
      (`KismetMaterialLibrary.SetVectorParameterValue` "/Game/TrailSystem/Blueprints/MPC_CustomTrails.MPC_CustomTrails" "PlayerLocation" (`KismetMathLibrary.Conv_VectorToLinearColor` (`Actor.K2_GetActorLocation` (`GameplayStatics.GetPlayerCharacter` 0))))
      (`KismetMaterialLibrary.SetVectorParameterValue` "/Game/TrailSystem/Blueprints/MPC_CustomTrails.MPC_CustomTrails" "PrevPlayerLocation" (`KismetMathLibrary.Conv_VectorToLinearColor` (`self.CachedPlayerLocation`)))
      (`KismetMaterialLibrary.SetVectorParameterValue` "/Game/TrailSystem/Blueprints/MPC_CustomTrails.MPC_CustomTrails" "PointLocation" (`KismetMathLibrary.Conv_VectorToLinearColor` (`self.K2_GetComponentLocation`)))
      (`KismetMaterialLibrary.SetVectorParameterValue` "/Game/TrailSystem/Blueprints/MPC_CustomTrails.MPC_CustomTrails" "PrevPointLocation" (`KismetMathLibrary.Conv_VectorToLinearColor` (`self.CachedLocation`)))
      (`KismetMaterialLibrary.SetScalarParameterValue` "/Game/TrailSystem/Blueprints/MPC_CustomTrails.MPC_CustomTrails" "PlayerYaw" (- (/ (+ _returnvalue_yaw 180.0) 180.0) 0.5))
      (`KismetMaterialLibrary.SetScalarParameterValue` "/Game/TrailSystem/Blueprints/MPC_CustomTrails.MPC_CustomTrails" "PrevPlayerYaw" (`self.CachedYaw`)))
    (:`then_1`
      (`KismetRenderingLibrary.DrawMaterialToRenderTarget` "/Game/TrailSystem/Blueprints/RT_Trails.RT_Trails" "/Game/Blueprint/PaintSystem/M_Rect.M_Rect"))
    (:`then_2`
      (`self.UpdateCache`))))

(fn `UpdateCache`
  (bind (_returnvalue_roll _returnvalue_pitch _returnvalue_yaw) (`KismetMathLibrary.BreakRotator` (`self.K2_GetComponentRotation`)))
  (set `self.CachedLocation` (`self.K2_GetComponentLocation`))
  (set `self.CachedYaw` (- (/ (+ _returnvalue_yaw 180.0) 180.0) 0.5))
  (set `self.CachedPlayerLocation` (`Actor.K2_GetActorLocation` (`GameplayStatics.GetPlayerCharacter` 0))))