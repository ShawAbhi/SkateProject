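; BP_TrackManager is a race-track actor that, when ManuallyPlaced is set, fits itself to the landscape in its construction script.
; SnapToLandscape line-traces vertically on a custom channel and returns the impact point, which becomes the actor's location.
; It then traces at each spline point and adds a scaled box component at the hit.
; The spline points themselves stay unmoved, and there is no active runtime logic.
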(fn `SnapToLandscape`
  (params (InputPin :type "Vector Structure") (DrawDebugType :type "EDrawDebugTrace Enum" :default "None"))
  (returns (ImpactPoint :type "Vector Structure"))
  (bind (_outhit _returnvalue) (`KismetSystemLibrary.LineTraceSingle` :`Start` (+ InputPin (* (`KismetMathLibrary.Vector_Up`) 200000.0)) :`End` (+ InputPin (* (`KismetMathLibrary.Vector_Down`) 200000.0)) :`TraceChannel` "TraceTypeQuery3" :`DrawDebugType` DrawDebugType :`DrawTime` 0.1))
  (if _returnvalue
    _
    (else
      _))
  (return (`.ImpactPoint` (`GameplayStatics.BreakHitResult` _outhit))))

(fn `UserConstructionScript`
  (if (`self.ManuallyPlaced`)
    (bind _impactpoint (`self.SnapToLandscape` (`self.K2_GetActorLocation`)))
    (`self.K2_SetActorLocation` _impactpoint false true)
    (for _index (range (+ (`SplineComponent.GetNumberOfSplinePoints` (`self.Spline`)) 1))
      (bind _impactpoint_2 (`self.SnapToLandscape` (`SplineComponent.GetLocationAtSplinePoint` (`self.Spline`) _index "World") "ForDuration"))
      (bind _returnvalue (`AddComponent|NODE_AddBoxComponent-0` :`RelativeTransform` (`KismetMathLibrary.MakeTransform` (0.0 0.0 0.0) (struct) (10.0 10.0 10.0))))
      (`SceneComponent.K2_SetWorldLocation` _returnvalue _impactpoint_2 false true))))