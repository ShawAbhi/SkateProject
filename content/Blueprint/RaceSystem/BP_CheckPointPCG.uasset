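; Race checkpoint actor that can display a world marker on the HUD until the player reaches it.
; On BeginPlay, if CanShowMarker is set, it waits briefly, then registers its billboard as a marker with the HUD manager.
; The player character overlapping its box removes that marker.
; The construction script snaps the actor onto the surface below via a tall vertical visibility trace, keeping only its yaw rotation.
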(event `self.ReceiveBeginPlay`
  (if (`self.CanShowMarker`)
    (`KismetSystemLibrary.Delay` 1.0)
    (`/Game/ProHUDV2/Blueprints/Libraries/BPi_HUDManagerV2.AddOrUpdateWorldMarker` (`/Game/ProHUDV2/Blueprints/Libraries/BP_PHV2_Functions.GetHUDManager`) (`self.MaterialBillboard`) (`self.WorldMarkerInfo`))))

(event `self.Box.OnComponentBeginOverlap`
  (params (OverlappedComponent :type "PrimitiveComponent Object Reference") (OtherActor :type "Actor Object Reference") (OtherComp :type "PrimitiveComponent Object Reference") (OtherBodyIndex :type Integer) (bFromSweep :type Boolean) (SweepResult :type "HitResult Structure (by ref)"))
  (if (== OtherActor (`GameplayStatics.GetPlayerCharacter` 0))
    (`/Game/ProHUDV2/Blueprints/Libraries/BPi_HUDManagerV2.RemoveWorldMarker` (`/Game/ProHUDV2/Blueprints/Libraries/BP_PHV2_Functions.GetHUDManager`) (`self.MaterialBillboard`))))

(fn `KeepActorOnLandscape`
  (bind _returnvalue (`self.K2_GetActorLocation`))
  (bind (_returnvalue_roll _returnvalue_pitch _returnvalue_yaw) (`KismetMathLibrary.BreakRotator` (`self.K2_GetActorRotation`)))
  (bind (_outhit _returnvalue_2) (`KismetSystemLibrary.LineTraceSingle` (+ _returnvalue (* (`KismetMathLibrary.Vector_Up`) 200000.0)) (+ _returnvalue (* (`KismetMathLibrary.Vector_Down`) 200000.0)) "TraceTypeQuery1"))
  (if _returnvalue_2
    (`self.K2_SetActorLocation` (`.ImpactPoint` (`GameplayStatics.BreakHitResult` _outhit)) false true)
    (`self.K2_SetActorRotation` (`KismetMathLibrary.MakeRotator` 0.0 0.0 _returnvalue_yaw))))

(fn `UserConstructionScript`
  (`self.KeepActorOnLandscape`))