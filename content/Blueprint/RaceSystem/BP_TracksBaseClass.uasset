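; Base race track Blueprint that manages an ordered series of BP_CheckPointPCG checkpoints placed as child actor components.
; The construction script sets each checkpoint's index from its component's first tag and refreshes its label.
; At BeginPlay it maps checkpoints by that tag, registers itself as their manager, then shows the first marker after a short delay.
; CheckpointReached advances to the next marker, flagging completion when none remains.
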(event Custom|CheckpointReached
  (Variables|Default|SetCompletedIndex (+ (Variables|Default|GetCompletedIndex) 1))
  (CallFunction|NextCheckpoint))

(event Custom|NextCheckpoint
  (bind _checkpointsmap (Variables|Default|GetCheckpointsMap))
  (bind _completedindex (Variables|Default|GetCompletedIndex))
  (bind (_value _returnvalue) (Utilities|Map|Find _checkpointsmap _completedindex))
  (if _returnvalue
    (Default|ShowMarker _value)
    (else
      (Variables|Default|SetCheckpointsCompleted true))))

(event EventBeginPlay
  (for _array_element (Actor|GetComponentsByClass "/Script/Engine.ChildActorComponent")
    (bind _asbp_check_point_pcg (Utilities|Casting|CastToBP_CheckPointPCG (Variables|/Script/Engine.ChildActorComponent|GetChildActor _array_element)))
    (Utilities|Map|Add (Variables|Default|GetCheckpointsMap) (Math|Conversions|ToInteger(Byte) (Utilities|String|ToString(Name) (Utilities|Array|Get(acopy) (Variables|/Script/Engine.ActorComponent|GetComponentTags _array_element)))) _asbp_check_point_pcg)
    (Variables|/Game/Blueprint/RaceSystem/BP_CheckPointPCG.BP_CheckPointPCG_C|SetManagerRef _asbp_check_point_pcg self))
  (Utilities|FlowControl|Delay 1.0)
  (CallFunction|NextCheckpoint))

(fn ConstructionScript
  (CallFunction|UpdateIndexes))

(fn UpdateIndexes
  (for _array_element (Actor|GetComponentsByClass "/Script/Engine.ChildActorComponent")
    (bind _asbp_check_point_pcg (Utilities|Casting|CastToBP_CheckPointPCG (Variables|/Script/Engine.ChildActorComponent|GetChildActor _array_element)))
    (Variables|/Game/Blueprint/RaceSystem/BP_CheckPointPCG.BP_CheckPointPCG_C|SetIndex _asbp_check_point_pcg (Math|Conversions|ToInteger(Byte) (Utilities|String|ToString(Name) (Utilities|Array|Get(acopy) (Variables|/Script/Engine.ActorComponent|GetComponentTags _array_element)))))
    (Default|UpdateText _asbp_check_point_pcg)))