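; BP_TargetActor is an actor in the PCG folder that snaps itself vertically onto the surface at its location.
; Its construction script calls KeepActorOnLandscape, which line-traces the Visibility channel from far above to far below the actor and teleports it to the impact point.
; The trace does not filter for landscape, so any blocking surface can catch it, and the event graph has no active logic.
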(event EventBeginPlay)

(event Collision|EventActorBeginOverlap
  (params (OtherActor :type Actor%20Object%20Reference)))

(event EventTick
  (params (DeltaSeconds :type Float%20%28single-precision%29)))

(fn ConstructionScript
  (CallFunction|KeepActoronLandscape))

(fn KeepActoronLandscape
  (bind _returnvalue (Transformation|GetActorLocation))
  (bind _returnvalue_2 (Math|Float|MakeLiteralFloat 2e+05))
  (bind (_outhit _returnvalue_3) (Collision|LineTraceByChannel (+ _returnvalue (* (Math|Vector|VectorUp) _returnvalue_2)) (+ _returnvalue (* (Math|Vector|VectorDown) _returnvalue_2)) "TraceTypeQuery1" false 0 "None"))
  (if _returnvalue_3
    (Transformation|SetActorLocation (.ImpactPoint (Collision|BreakHitResult _outhit)) false true)))