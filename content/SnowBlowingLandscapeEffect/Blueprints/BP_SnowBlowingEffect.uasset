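; Decal actor that renders a blowing snow effect, with a selectable preset material and adjustable box size.
; Construction script and BeginPlay both apply the decal material and scale, then run all six preset functions regardless of selection.
; Each function copies its flowmap, noise, deform, fade and color variables into its own Material Parameter Collection.
; Some writes target mismatched names: Preset 3's deform speeds and Presets 4 and 6's Phase 1 time.
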(event `self.ReceiveBeginPlay`
  (`DecalComponent.SetDecalMaterial` (`self.SnowDecal`) (`self.Preset Selection`))
  (`SceneComponent.SetWorldScale3D` (`self.SnowDecal`) (`self.BoxEffectSize`))
  (`self.Preset1`)
  (`self.Preset2`)
  (`self.Preset 3`)
  (`self.Preset 4`)
  (`self.Preset 5`)
  (`self.Preset 6`))

(fn `Preset 3`
  (`KismetMaterialLibrary.SetScalarParameterValue` "/Game/SnowBlowingLandscapeEffect/Materials/MPC_Preset_3.MPC_Preset_3" "CameraFadeDistance3" (`self.CameraFadeDistance3`))
  (`KismetMaterialLibrary.SetScalarParameterValue` "/Game/SnowBlowingLandscapeEffect/Materials/MPC_Preset_3.MPC_Preset_3" "Phase 1 UVs Flowmap3" (`self.Phase 1 UVs Flowmap3`))
  (`KismetMaterialLibrary.SetScalarParameterValue` "/Game/SnowBlowingLandscapeEffect/Materials/MPC_Preset_3.MPC_Preset_3" "Phase 1 UVs Noise3" (`self.Phase 1 UVs Noise3`))
  (`KismetMaterialLibrary.SetScalarParameterValue` "/Game/SnowBlowingLandscapeEffect/Materials/MPC_Preset_3.MPC_Preset_3" "Phase 1 FlowStrenght3" (`self.Phase 1 FlowStrenght3`))
  (`KismetMaterialLibrary.SetScalarParameterValue` "/Game/SnowBlowingLandscapeEffect/Materials/MPC_Preset_3.MPC_Preset_3" "Phase 1 Time3" (`self.Phase 1 Time3`))
  (`KismetMaterialLibrary.SetScalarParameterValue` "/Game/SnowBlowingLandscapeEffect/Materials/MPC_Preset_3.MPC_Preset_3" "Phase 1 X NoiseSpeed3" (`self.Phase 1 X NoiseSpeed3`))
  (`KismetMaterialLibrary.SetScalarParameterValue` "/Game/SnowBlowingLandscapeEffect/Materials/MPC_Preset_3.MPC_Preset_3" "Phase 1 X NoiseSpeed3" (`self.Phase 1 Y NoiseSpeed3`))
  (`KismetMaterialLibrary.SetScalarParameterValue` "/Game/SnowBlowingLandscapeEffect/Materials/MPC_Preset_3.MPC_Preset_3" "Phase 1 Contrast3" (`self.Phase 1 Contrast3`))
  (`KismetMaterialLibrary.SetScalarParameterValue` "/Game/SnowBlowingLandscapeEffect/Materials/MPC_Preset_3.MPC_Preset_3" "Phase 1 Opacity3" (`self.Phase 1 Opacity3`))
  (`KismetMaterialLibrary.SetScalarParameterValue` "/Game/SnowBlowingLandscapeEffect/Materials/MPC_Preset_3.MPC_Preset_3" "Phase 1 X NoiseSpeed3" (`self.Deform X NoiseSpeed3`))
  (`KismetMaterialLibrary.SetScalarParameterValue` "/Game/SnowBlowingLandscapeEffect/Materials/MPC_Preset_3.MPC_Preset_3" "Phase 1 Y NoiseSpeed3" (`self.Deform Y NoiseSpeed3`))
  (`KismetMaterialLibrary.SetScalarParameterValue` "/Game/SnowBlowingLandscapeEffect/Materials/MPC_Preset_3.MPC_Preset_3" "DeformUVs3" (`self.DeformUVs3`))
  (`KismetMaterialLibrary.SetScalarParameterValue` "/Game/SnowBlowingLandscapeEffect/Materials/MPC_Preset_3.MPC_Preset_3" "DeformContrast3" (`self.DeformContrast3`))
  (`KismetMaterialLibrary.SetScalarParameterValue` "/Game/SnowBlowingLandscapeEffect/Materials/MPC_Preset_3.MPC_Preset_3" "DeformOpacity3" (`self.DeformOpacity3`))
  (`KismetMaterialLibrary.SetScalarParameterValue` "/Game/SnowBlowingLandscapeEffect/Materials/MPC_Preset_3.MPC_Preset_3" "Phase 2 Uvs Flowmap3" (`self.Phase 2 Uvs Flowmap3`))
  (`KismetMaterialLibrary.SetScalarParameterValue` "/Game/SnowBlowingLandscapeEffect/Materials/MPC_Preset_3.MPC_Preset_3" "Phase 2 Uvs Noise3" (`self.Phase 2 Uvs Noise3`))
  (`KismetMaterialLibrary.SetScalarParameterValue` "/Game/SnowBlowingLandscapeEffect/Materials/MPC_Preset_3.MPC_Preset_3" "Phase 2 FlowStrenght3" (`self.Phase 2 FlowStrenght3`))
  (`KismetMaterialLibrary.SetScalarParameterValue` "/Game/SnowBlowingLandscapeEffect/Materials/MPC_Preset_3.MPC_Preset_3" "Phase 2 Time3" (`self.Phase 2 Time3`))
  (`KismetMaterialLibrary.SetScalarParameterValue` "/Game/SnowBlowingLandscapeEffect/Materials/MPC_Preset_3.MPC_Preset_3" "Phase 2 X NoiseSpeed3" (`self.Phase 2 X NoiseSpeed3`))
  (`KismetMaterialLibrary.SetScalarParameterValue` "/Game/SnowBlowingLandscapeEffect/Materials/MPC_Preset_3.MPC_Preset_3" "Phase 2 Y NoiseSpeed3" (`self.Phase 2 Y NoiseSpeed3`))
  (`KismetMaterialLibrary.SetScalarParameterValue` "/Game/SnowBlowingLandscapeEffect/Materials/MPC_Preset_3.MPC_Preset_3" "Phase 2 Contrast3" (`self.Phase 2 Contrast3`))
  (`KismetMaterialLibrary.SetScalarParameterValue` "/Game/SnowBlowingLandscapeEffect/Materials/MPC_Preset_3.MPC_Preset_3" "Phase 2 Opacity3" (`self.Phase 2 Opacity3`))
  (`KismetMaterialLibrary.SetScalarParameterValue` "/Game/SnowBlowingLandscapeEffect/Materials/MPC_Preset_3.MPC_Preset_3" "Phase 1 DistortionStart3" (`self.Phase 1 DistortionStartRange3`))
  (`KismetMaterialLibrary.SetScalarParameterValue` "/Game/SnowBlowingLandscapeEffect/Materials/MPC_Preset_3.MPC_Preset_3" "Phase 1 DistortionEnd3" (`self.Phase 1 DistortionEndRange3`))
  (`KismetMaterialLibrary.SetVectorParameterValue` "/Game/SnowBlowingLandscapeEffect/Materials/MPC_Preset_3.MPC_Preset_3" "SnowColor3" (`self.SnowColor3`)))

(fn `Preset 4`
  (`KismetMaterialLibrary.SetScalarParameterValue` "/Game/SnowBlowingLandscapeEffect/Materials/MPC_Preset_4.MPC_Preset_4" "CameraFadeDistance4" (`self.CameraFadeDistance4`))
  (`KismetMaterialLibrary.SetScalarParameterValue` "/Game/SnowBlowingLandscapeEffect/Materials/MPC_Preset_4.MPC_Preset_4" "Phase 1 UVs Flowmap4" (`self.Phase 1 UVs Flowmap4`))
  (`KismetMaterialLibrary.SetScalarParameterValue` "/Game/SnowBlowingLandscapeEffect/Materials/MPC_Preset_4.MPC_Preset_4" "Phase 1 UVs Noise4" (`self.Phase 1 UVs Noise4`))
  (`KismetMaterialLibrary.SetScalarParameterValue` "/Game/SnowBlowingLandscapeEffect/Materials/MPC_Preset_4.MPC_Preset_4" "Phase 1 FlowStrenght4" (`self.Phase 1 FlowStrenght4`))
  (`KismetMaterialLibrary.SetScalarParameterValue` "/Game/SnowBlowingLandscapeEffect/Materials/MPC_Preset_4.MPC_Preset_4" "Phase 2 Time4" (`self.Phase 1 Time4`))
  (`KismetMaterialLibrary.SetScalarParameterValue` "/Game/SnowBlowingLandscapeEffect/Materials/MPC_Preset_4.MPC_Preset_4" "Phase 1 X NoiseSpeed4" (`self.Phase 1 X NoiseSpeed4`))
  (`KismetMaterialLibrary.SetScalarParameterValue` "/Game/SnowBlowingLandscapeEffect/Materials/MPC_Preset_4.MPC_Preset_4" "Phase 1 Y NoiseSpeed4" (`self.Phase 1 Y NoiseSpeed4`))
  (`KismetMaterialLibrary.SetScalarParameterValue` "/Game/SnowBlowingLandscapeEffect/Materials/MPC_Preset_4.MPC_Preset_4" "Phase 1 Contrast4" (`self.Phase 1 Contrast4`))
  (`KismetMaterialLibrary.SetScalarParameterValue` "/Game/SnowBlowingLandscapeEffect/Materials/MPC_Preset_4.MPC_Preset_4" "Phase 1 Opacity4" (`self.Phase 1 Opacity4`))
  (`KismetMaterialLibrary.SetScalarParameterValue` "/Game/SnowBlowingLandscapeEffect/Materials/MPC_Preset_4.MPC_Preset_4" "Deform X NoiseSpeed4" (`self.Deform X NoiseSpeed4`))
  (`KismetMaterialLibrary.SetScalarParameterValue` "/Game/SnowBlowingLandscapeEffect/Materials/MPC_Preset_4.MPC_Preset_4" "Deform Y NoiseSpeed4" (`self.Deform Y NoiseSpeed4`))
  (`KismetMaterialLibrary.SetScalarParameterValue` "/Game/SnowBlowingLandscapeEffect/Materials/MPC_Preset_4.MPC_Preset_4" "DeformUVs4" (`self.DeformUVs4`))
  (`KismetMaterialLibrary.SetScalarParameterValue` "/Game/SnowBlowingLandscapeEffect/Materials/MPC_Preset_4.MPC_Preset_4" "DeformContrast4" (`self.DeformContrast4`))
  (`KismetMaterialLibrary.SetScalarParameterValue` "/Game/SnowBlowingLandscapeEffect/Materials/MPC_Preset_4.MPC_Preset_4" "DeformOpacity4" (`self.DeformOpacity4`))
  (`KismetMaterialLibrary.SetScalarParameterValue` "/Game/SnowBlowingLandscapeEffect/Materials/MPC_Preset_4.MPC_Preset_4" "Phase 2 Uvs Flowmap4" (`self.Phase 2 Uvs Flowmap4`))
  (`KismetMaterialLibrary.SetScalarParameterValue` "/Game/SnowBlowingLandscapeEffect/Materials/MPC_Preset_4.MPC_Preset_4" "Phase 2 Uvs Noise4" (`self.Phase 2 Uvs Noise4`))
  (`KismetMaterialLibrary.SetScalarParameterValue` "/Game/SnowBlowingLandscapeEffect/Materials/MPC_Preset_4.MPC_Preset_4" "Phase 2 FlowStrenght4" (`self.Phase 2 FlowStrenght4`))
  (`KismetMaterialLibrary.SetScalarParameterValue` "/Game/SnowBlowingLandscapeEffect/Materials/MPC_Preset_4.MPC_Preset_4" "Phase 2 Time4" (`self.Phase 2 Time4`))
  (`KismetMaterialLibrary.SetScalarParameterValue` "/Game/SnowBlowingLandscapeEffect/Materials/MPC_Preset_4.MPC_Preset_4" "Phase 2 X NoiseSpeed4" (`self.Phase 2 X NoiseSpeed4`))
  (`KismetMaterialLibrary.SetScalarParameterValue` "/Game/SnowBlowingLandscapeEffect/Materials/MPC_Preset_4.MPC_Preset_4" "Phase 2 Y NoiseSpeed4" (`self.Phase 2 Y NoiseSpeed4`))
  (`KismetMaterialLibrary.SetScalarParameterValue` "/Game/SnowBlowingLandscapeEffect/Materials/MPC_Preset_4.MPC_Preset_4" "Phase 2 Contrast4" (`self.Phase 2 Contrast4`))
  (`KismetMaterialLibrary.SetScalarParameterValue` "/Game/SnowBlowingLandscapeEffect/Materials/MPC_Preset_4.MPC_Preset_4" "Phase 2 Opacity4" (`self.Phase 2 Opacity4`))
  (`KismetMaterialLibrary.SetScalarParameterValue` "/Game/SnowBlowingLandscapeEffect/Materials/MPC_Preset_4.MPC_Preset_4" "Phase 1 DistortionStart4" (`self.Phase 1 DistortionStartRange4`))
  (`KismetMaterialLibrary.SetScalarParameterValue` "/Game/SnowBlowingLandscapeEffect/Materials/MPC_Preset_4.MPC_Preset_4" "Phase 1 DistortionEnd4" (`self.Phase 1 DistortionEndRange4`))
  (`KismetMaterialLibrary.SetVectorParameterValue` "/Game/SnowBlowingLandscapeEffect/Materials/MPC_Preset_4.MPC_Preset_4" "SnowColor4" (`self.SnowColor4`)))

(fn `Preset 5`
  (`KismetMaterialLibrary.SetScalarParameterValue` "/Game/SnowBlowingLandscapeEffect/Materials/MPC_Preset_5.MPC_Preset_5" "CameraFadeDistance5" (`self.CameraFadeDistance5`))
  (`KismetMaterialLibrary.SetScalarParameterValue` "/Game/SnowBlowingLandscapeEffect/Materials/MPC_Preset_5.MPC_Preset_5" "Phase 1 UVs Flowmap5" (`self.Phase 1 UVs Flowmap5`))
  (`KismetMaterialLibrary.SetScalarParameterValue` "/Game/SnowBlowingLandscapeEffect/Materials/MPC_Preset_5.MPC_Preset_5" "Phase 1 UVs Noise5" (`self.Phase 1 UVs Noise5`))
  (`KismetMaterialLibrary.SetScalarParameterValue` "/Game/SnowBlowingLandscapeEffect/Materials/MPC_Preset_5.MPC_Preset_5" "Phase 1 FlowStrenght5" (`self.Phase 1 FlowStrenght5`))
  (`KismetMaterialLibrary.SetScalarParameterValue` "/Game/SnowBlowingLandscapeEffect/Materials/MPC_Preset_5.MPC_Preset_5" "Phase 1 DistortionStart5" (`self.Phase 1 DistortionStartRange5`))
  (`KismetMaterialLibrary.SetScalarParameterValue` "/Game/SnowBlowingLandscapeEffect/Materials/MPC_Preset_5.MPC_Preset_5" "Phase 1 DistortionEnd5" (`self.Phase 1 DistortionEndRange5`))
  (`KismetMaterialLibrary.SetScalarParameterValue` "/Game/SnowBlowingLandscapeEffect/Materials/MPC_Preset_5.MPC_Preset_5" "Phase 1 Time5" (`self.Phase 1 Time5`))
  (`KismetMaterialLibrary.SetScalarParameterValue` "/Game/SnowBlowingLandscapeEffect/Materials/MPC_Preset_5.MPC_Preset_5" "Phase 1 X NoiseSpeed5" (`self.Phase 1 X NoiseSpeed5`))
  (`KismetMaterialLibrary.SetScalarParameterValue` "/Game/SnowBlowingLandscapeEffect/Materials/MPC_Preset_5.MPC_Preset_5" "Phase 1 Y NoiseSpeed5" (`self.Phase 1 Y NoiseSpeed5`))
  (`KismetMaterialLibrary.SetScalarParameterValue` "/Game/SnowBlowingLandscapeEffect/Materials/MPC_Preset_5.MPC_Preset_5" "Phase 1 Contrast5" (`self.Phase 1 Contrast5`))
  (`KismetMaterialLibrary.SetScalarParameterValue` "/Game/SnowBlowingLandscapeEffect/Materials/MPC_Preset_5.MPC_Preset_5" "Phase 1 Opacity5" (`self.Phase 1 Opacity5`))
  (`KismetMaterialLibrary.SetScalarParameterValue` "/Game/SnowBlowingLandscapeEffect/Materials/MPC_Preset_5.MPC_Preset_5" "Deform X NoiseSpeed5" (`self.Deform X NoiseSpeed5`))
  (`KismetMaterialLibrary.SetScalarParameterValue` "/Game/SnowBlowingLandscapeEffect/Materials/MPC_Preset_5.MPC_Preset_5" "Deform Y NoiseSpeed5" (`self.Deform Y NoiseSpeed5`))
  (`KismetMaterialLibrary.SetScalarParameterValue` "/Game/SnowBlowingLandscapeEffect/Materials/MPC_Preset_5.MPC_Preset_5" "DeformUVs5" (`self.DeformUVs5`))
  (`KismetMaterialLibrary.SetScalarParameterValue` "/Game/SnowBlowingLandscapeEffect/Materials/MPC_Preset_5.MPC_Preset_5" "DeformContrast5" (`self.DeformContrast5`))
  (`KismetMaterialLibrary.SetScalarParameterValue` "/Game/SnowBlowingLandscapeEffect/Materials/MPC_Preset_5.MPC_Preset_5" "DeformOpacity5" (`self.DeformOpacity5`))
  (`KismetMaterialLibrary.SetScalarParameterValue` "/Game/SnowBlowingLandscapeEffect/Materials/MPC_Preset_5.MPC_Preset_5" "Phase 2 Uvs Flowmap5" (`self.Phase 2 Uvs Flowmap5`))
  (`KismetMaterialLibrary.SetScalarParameterValue` "/Game/SnowBlowingLandscapeEffect/Materials/MPC_Preset_5.MPC_Preset_5" "Phase 2 Uvs Noise5" (`self.Phase 2 Uvs Noise5`))
  (`KismetMaterialLibrary.SetScalarParameterValue` "/Game/SnowBlowingLandscapeEffect/Materials/MPC_Preset_5.MPC_Preset_5" "Phase 2 FlowStrenght5" (`self.Phase 2 FlowStrenght5`))
  (`KismetMaterialLibrary.SetScalarParameterValue` "/Game/SnowBlowingLandscapeEffect/Materials/MPC_Preset_5.MPC_Preset_5" "Phase 2 Time5" (`self.Phase 2 Time5`))
  (`KismetMaterialLibrary.SetScalarParameterValue` "/Game/SnowBlowingLandscapeEffect/Materials/MPC_Preset_5.MPC_Preset_5" "Phase 2 X NoiseSpeed5" (`self.Phase 2 X NoiseSpeed5`))
  (`KismetMaterialLibrary.SetScalarParameterValue` "/Game/SnowBlowingLandscapeEffect/Materials/MPC_Preset_5.MPC_Preset_5" "Phase 2 Y NoiseSpeed5" (`self.Phase 2 Y NoiseSpeed5`))
  (`KismetMaterialLibrary.SetScalarParameterValue` "/Game/SnowBlowingLandscapeEffect/Materials/MPC_Preset_5.MPC_Preset_5" "Phase 2 Contrast5" (`self.Phase 2 Contrast5`))
  (`KismetMaterialLibrary.SetScalarParameterValue` "/Game/SnowBlowingLandscapeEffect/Materials/MPC_Preset_5.MPC_Preset_5" "Phase 2 Opacity5" (`self.Phase 2 Opacity5`))
  (`KismetMaterialLibrary.SetVectorParameterValue` "/Game/SnowBlowingLandscapeEffect/Materials/MPC_Preset_5.MPC_Preset_5" "SnowColor5" (`self.SnowColor5`)))

(fn `Preset 6`
  (`KismetMaterialLibrary.SetScalarParameterValue` "/Game/SnowBlowingLandscapeEffect/Materials/MPC_Preset_6.MPC_Preset_6" "CameraFadeDistance6" (`self.CameraFadeDistance6`))
  (`KismetMaterialLibrary.SetScalarParameterValue` "/Game/SnowBlowingLandscapeEffect/Materials/MPC_Preset_6.MPC_Preset_6" "Phase 1 UVs Flowmap6" (`self.Phase 1 UVs Flowmap6`))
  (`KismetMaterialLibrary.SetScalarParameterValue` "/Game/SnowBlowingLandscapeEffect/Materials/MPC_Preset_6.MPC_Preset_6" "Phase 1 UVs Noise6" (`self.Phase 1 UVs Noise6`))
  (`KismetMaterialLibrary.SetScalarParameterValue` "/Game/SnowBlowingLandscapeEffect/Materials/MPC_Preset_6.MPC_Preset_6" "Phase 1 FlowStrenght6" (`self.Phase 1 FlowStrenght6`))
  (`KismetMaterialLibrary.SetScalarParameterValue` "/Game/SnowBlowingLandscapeEffect/Materials/MPC_Preset_6.MPC_Preset_6" "Phase 1 DistortionStart6" (`self.Phase 1 DistortionStartRange6`))
  (`KismetMaterialLibrary.SetScalarParameterValue` "/Game/SnowBlowingLandscapeEffect/Materials/MPC_Preset_6.MPC_Preset_6" "Phase 1 DistortionEnd6" (`self.Phase 1 DistortionEndRange6`))
  (`KismetMaterialLibrary.SetScalarParameterValue` "/Game/SnowBlowingLandscapeEffect/Materials/MPC_Preset_6.MPC_Preset_6" "Phase 2 Time6" (`self.Phase 1 Time6`))
  (`KismetMaterialLibrary.SetScalarParameterValue` "/Game/SnowBlowingLandscapeEffect/Materials/MPC_Preset_6.MPC_Preset_6" "Phase 1 X NoiseSpeed6" (`self.Phase 1 X NoiseSpeed6`))
  (`KismetMaterialLibrary.SetScalarParameterValue` "/Game/SnowBlowingLandscapeEffect/Materials/MPC_Preset_6.MPC_Preset_6" "Phase 1 Y NoiseSpeed6" (`self.Phase 1 Y NoiseSpeed6`))
  (`KismetMaterialLibrary.SetScalarParameterValue` "/Game/SnowBlowingLandscapeEffect/Materials/MPC_Preset_6.MPC_Preset_6" "Phase 1 Contrast6" (`self.Phase 1 Contrast6`))
  (`KismetMaterialLibrary.SetScalarParameterValue` "/Game/SnowBlowingLandscapeEffect/Materials/MPC_Preset_6.MPC_Preset_6" "Phase 1 Opacity6" (`self.Phase 1 Opacity6`))
  (`KismetMaterialLibrary.SetScalarParameterValue` "/Game/SnowBlowingLandscapeEffect/Materials/MPC_Preset_6.MPC_Preset_6" "Deform X NoiseSpeed6" (`self.Deform X NoiseSpeed6`))
  (`KismetMaterialLibrary.SetScalarParameterValue` "/Game/SnowBlowingLandscapeEffect/Materials/MPC_Preset_6.MPC_Preset_6" "DeformUVs6" (`self.DeformUVs6`))
  (`KismetMaterialLibrary.SetScalarParameterValue` "/Game/SnowBlowingLandscapeEffect/Materials/MPC_Preset_6.MPC_Preset_6" "DeformContrast6" (`self.DeformContrast6`))
  (`KismetMaterialLibrary.SetScalarParameterValue` "/Game/SnowBlowingLandscapeEffect/Materials/MPC_Preset_6.MPC_Preset_6" "DeformOpacity6" (`self.DeformOpacity6`))
  (`KismetMaterialLibrary.SetScalarParameterValue` "/Game/SnowBlowingLandscapeEffect/Materials/MPC_Preset_6.MPC_Preset_6" "Phase 2 Uvs Flowmap6" (`self.Phase 2 Uvs Flowmap6`))
  (`KismetMaterialLibrary.SetScalarParameterValue` "/Game/SnowBlowingLandscapeEffect/Materials/MPC_Preset_6.MPC_Preset_6" "Phase 2 Uvs Noise6" (`self.Phase 2 Uvs Noise6`))
  (`KismetMaterialLibrary.SetScalarParameterValue` "/Game/SnowBlowingLandscapeEffect/Materials/MPC_Preset_6.MPC_Preset_6" "Phase 2 FlowStrenght6" (`self.Phase 2 FlowStrenght6`))
  (`KismetMaterialLibrary.SetScalarParameterValue` "/Game/SnowBlowingLandscapeEffect/Materials/MPC_Preset_6.MPC_Preset_6" "Phase 2 Time6" (`self.Phase 2 Time6`))
  (`KismetMaterialLibrary.SetScalarParameterValue` "/Game/SnowBlowingLandscapeEffect/Materials/MPC_Preset_6.MPC_Preset_6" "Phase 2 X NoiseSpeed6" (`self.Phase 2 X NoiseSpeed6`))
  (`KismetMaterialLibrary.SetScalarParameterValue` "/Game/SnowBlowingLandscapeEffect/Materials/MPC_Preset_6.MPC_Preset_6" "Phase 2 Y NoiseSpeed6" (`self.Phase 2 Y NoiseSpeed6`))
  (`KismetMaterialLibrary.SetScalarParameterValue` "/Game/SnowBlowingLandscapeEffect/Materials/MPC_Preset_6.MPC_Preset_6" "Phase 2 Contrast6" (`self.Phase 2 Contrast6`))
  (`KismetMaterialLibrary.SetScalarParameterValue` "/Game/SnowBlowingLandscapeEffect/Materials/MPC_Preset_6.MPC_Preset_6" "Phase 2 Opacity6" (`self.Phase 2 Opacity6`))
  (`KismetMaterialLibrary.SetScalarParameterValue` "/Game/SnowBlowingLandscapeEffect/Materials/MPC_Preset_6.MPC_Preset_6" "Deform Y NoiseSpeed6" (`self.Deform Y NoiseSpeed6`))
  (`KismetMaterialLibrary.SetVectorParameterValue` "/Game/SnowBlowingLandscapeEffect/Materials/MPC_Preset_6.MPC_Preset_6" "SnowColor6" (`self.SnowColor6`)))

(fn `Preset1`
  (`KismetMaterialLibrary.SetScalarParameterValue` "/Game/SnowBlowingLandscapeEffect/Materials/MPC_Preset_1.MPC_Preset_1" "CameraFadeDistance1" (`self.CameraFadeDistance1`))
  (`KismetMaterialLibrary.SetScalarParameterValue` "/Game/SnowBlowingLandscapeEffect/Materials/MPC_Preset_1.MPC_Preset_1" "Phase 1 UVs Flowmap1" (`self.Phase 1 UVs Flowmap1`))
  (`KismetMaterialLibrary.SetScalarParameterValue` "/Game/SnowBlowingLandscapeEffect/Materials/MPC_Preset_1.MPC_Preset_1" "Phase 1 FlowStrenght1" (`self.Phase 1 FlowStrenght1`))
  (`KismetMaterialLibrary.SetScalarParameterValue` "/Game/SnowBlowingLandscapeEffect/Materials/MPC_Preset_1.MPC_Preset_1" "Phase 1 UVs Noise1" (`self.Phase 1 UVs Noise1`))
  (`KismetMaterialLibrary.SetScalarParameterValue` "/Game/SnowBlowingLandscapeEffect/Materials/MPC_Preset_1.MPC_Preset_1" "Phase 1 X NoiseSpeed1" (`self.Phase 1 X NoiseSpeed1`))
  (`KismetMaterialLibrary.SetScalarParameterValue` "/Game/SnowBlowingLandscapeEffect/Materials/MPC_Preset_1.MPC_Preset_1" "Phase 1 Y NoiseSpeed1" (`self.Phase 1 Y NoiseSpeed1`))
  (`KismetMaterialLibrary.SetScalarParameterValue` "/Game/SnowBlowingLandscapeEffect/Materials/MPC_Preset_1.MPC_Preset_1" "Phase 1 Time1" (`self.Phase 1 Time1`))
  (`KismetMaterialLibrary.SetScalarParameterValue` "/Game/SnowBlowingLandscapeEffect/Materials/MPC_Preset_1.MPC_Preset_1" "Phase 1 Contrast1" (`self.Phase 1 Contrast1`))
  (`KismetMaterialLibrary.SetScalarParameterValue` "/Game/SnowBlowingLandscapeEffect/Materials/MPC_Preset_1.MPC_Preset_1" "Phase 1 Opacity1" (`self.Phase 1 Opacity1`))
  (`KismetMaterialLibrary.SetScalarParameterValue` "/Game/SnowBlowingLandscapeEffect/Materials/MPC_Preset_1.MPC_Preset_1" "DeformUVs1" (`self.DeformUVs1`))
  (`KismetMaterialLibrary.SetScalarParameterValue` "/Game/SnowBlowingLandscapeEffect/Materials/MPC_Preset_1.MPC_Preset_1" "Deform X NoiseSpeed1" (`self.Deform X NoiseSpeed1`))
  (`KismetMaterialLibrary.SetScalarParameterValue` "/Game/SnowBlowingLandscapeEffect/Materials/MPC_Preset_1.MPC_Preset_1" "Deform Y NoiseSpeed1" (`self.Deform Y NoiseSpeed1`))
  (`KismetMaterialLibrary.SetScalarParameterValue` "/Game/SnowBlowingLandscapeEffect/Materials/MPC_Preset_1.MPC_Preset_1" "DeformContrast1" (`self.DeformContrast1`))
  (`KismetMaterialLibrary.SetScalarParameterValue` "/Game/SnowBlowingLandscapeEffect/Materials/MPC_Preset_1.MPC_Preset_1" "DeformOpacity1" (`self.DeformOpacity1`))
  (`KismetMaterialLibrary.SetScalarParameterValue` "/Game/SnowBlowingLandscapeEffect/Materials/MPC_Preset_1.MPC_Preset_1" "Phase 2 Uvs Flowmap1" (`self.Phase 2 Uvs Flowmap1`))
  (`KismetMaterialLibrary.SetScalarParameterValue` "/Game/SnowBlowingLandscapeEffect/Materials/MPC_Preset_1.MPC_Preset_1" "Phase 2 FlowStrenght1" (`self.Phase 2 FlowStrenght1`))
  (`KismetMaterialLibrary.SetScalarParameterValue` "/Game/SnowBlowingLandscapeEffect/Materials/MPC_Preset_1.MPC_Preset_1" "Phase 2 Uvs Noise1" (`self.Phase 2 Uvs Noise1`))
  (`KismetMaterialLibrary.SetScalarParameterValue` "/Game/SnowBlowingLandscapeEffect/Materials/MPC_Preset_1.MPC_Preset_1" "Phase 2 X NoiseSpeed1" (`self.Phase 2 X NoiseSpeed1`))
  (`KismetMaterialLibrary.SetScalarParameterValue` "/Game/SnowBlowingLandscapeEffect/Materials/MPC_Preset_1.MPC_Preset_1" "Phase 2 Y NoiseSpeed1" (`self.Phase 2 Y NoiseSpeed1`))
  (`KismetMaterialLibrary.SetScalarParameterValue` "/Game/SnowBlowingLandscapeEffect/Materials/MPC_Preset_1.MPC_Preset_1" "Phase 2 Time1" (`self.Phase 2 Time1`))
  (`KismetMaterialLibrary.SetScalarParameterValue` "/Game/SnowBlowingLandscapeEffect/Materials/MPC_Preset_1.MPC_Preset_1" "Phase 2 Contrast1" (`self.Phase 2 Contrast1`))
  (`KismetMaterialLibrary.SetScalarParameterValue` "/Game/SnowBlowingLandscapeEffect/Materials/MPC_Preset_1.MPC_Preset_1" "Phase 2 Opacity1" (`self.Phase 2 Opacity1`))
  (`KismetMaterialLibrary.SetScalarParameterValue` "/Game/SnowBlowingLandscapeEffect/Materials/MPC_Preset_1.MPC_Preset_1" "Phase 1 DistortionStart1" (`self.Phase 1 DistortionStartRange1`))
  (`KismetMaterialLibrary.SetScalarParameterValue` "/Game/SnowBlowingLandscapeEffect/Materials/MPC_Preset_1.MPC_Preset_1" "Phase 1 DistortionEnd1" (`self.Phase 1 DistortionEndRange1`))
  (`KismetMaterialLibrary.SetVectorParameterValue` "/Game/SnowBlowingLandscapeEffect/Materials/MPC_Preset_1.MPC_Preset_1" "SnowColor" (`self.SnowColor`)))

(fn `Preset2`
  (`KismetMaterialLibrary.SetScalarParameterValue` "/Game/SnowBlowingLandscapeEffect/Materials/MPC_Preset_2.MPC_Preset_2" "CameraFadeDistance2" (`self.CameraFadeDistance2`))
  (`KismetMaterialLibrary.SetScalarParameterValue` "/Game/SnowBlowingLandscapeEffect/Materials/MPC_Preset_2.MPC_Preset_2" "Phase 1 UVs Flowmap2" (`self.Phase 1 UVs Flowmap2`))
  (`KismetMaterialLibrary.SetScalarParameterValue` "/Game/SnowBlowingLandscapeEffect/Materials/MPC_Preset_2.MPC_Preset_2" "Phase 1 FlowStrenght2" (`self.Phase 1 FlowStrenght2`))
  (`KismetMaterialLibrary.SetScalarParameterValue` "/Game/SnowBlowingLandscapeEffect/Materials/MPC_Preset_2.MPC_Preset_2" "Phase 1 UVs Noise2" (`self.Phase 1 UVs Noise2`))
  (`KismetMaterialLibrary.SetScalarParameterValue` "/Game/SnowBlowingLandscapeEffect/Materials/MPC_Preset_2.MPC_Preset_2" "Phase 1 X NoiseSpeed2" (`self.Phase 1 X NoiseSpeed2`))
  (`KismetMaterialLibrary.SetScalarParameterValue` "/Game/SnowBlowingLandscapeEffect/Materials/MPC_Preset_2.MPC_Preset_2" "Phase 1 Y NoiseSpeed2" (`self.Phase 1 Y NoiseSpeed2`))
  (`KismetMaterialLibrary.SetScalarParameterValue` "/Game/SnowBlowingLandscapeEffect/Materials/MPC_Preset_2.MPC_Preset_2" "Phase 1 Time2" (`self.Phase 1 Time2`))
  (`KismetMaterialLibrary.SetScalarParameterValue` "/Game/SnowBlowingLandscapeEffect/Materials/MPC_Preset_2.MPC_Preset_2" "Phase 1 Contrast2" (`self.Phase 1 Contrast2`))
  (`KismetMaterialLibrary.SetScalarParameterValue` "/Game/SnowBlowingLandscapeEffect/Materials/MPC_Preset_2.MPC_Preset_2" "Phase 1 Opacity2" (`self.Phase 1 Opacity2`))
  (`KismetMaterialLibrary.SetScalarParameterValue` "/Game/SnowBlowingLandscapeEffect/Materials/MPC_Preset_2.MPC_Preset_2" "DeformUVs2" (`self.DeformUVs2`))
  (`KismetMaterialLibrary.SetScalarParameterValue` "/Game/SnowBlowingLandscapeEffect/Materials/MPC_Preset_2.MPC_Preset_2" "Deform X NoiseSpeed2" (`self.Deform X NoiseSpeed2`))
  (`KismetMaterialLibrary.SetScalarParameterValue` "/Game/SnowBlowingLandscapeEffect/Materials/MPC_Preset_2.MPC_Preset_2" "Deform Y NoiseSpeed2" (`self.Deform Y NoiseSpeed2`))
  (`KismetMaterialLibrary.SetScalarParameterValue` "/Game/SnowBlowingLandscapeEffect/Materials/MPC_Preset_2.MPC_Preset_2" "DeformContrast2" (`self.DeformContrast2`))
  (`KismetMaterialLibrary.SetScalarParameterValue` "/Game/SnowBlowingLandscapeEffect/Materials/MPC_Preset_2.MPC_Preset_2" "DeformOpacity2" (`self.DeformOpacity2`))
  (`KismetMaterialLibrary.SetScalarParameterValue` "/Game/SnowBlowingLandscapeEffect/Materials/MPC_Preset_2.MPC_Preset_2" "Phase 2 Uvs Flowmap2" (`self.Phase 2 Uvs Flowmap2`))
  (`KismetMaterialLibrary.SetScalarParameterValue` "/Game/SnowBlowingLandscapeEffect/Materials/MPC_Preset_2.MPC_Preset_2" "Phase 2 FlowStrenght2" (`self.Phase 2 FlowStrenght2`))
  (`KismetMaterialLibrary.SetScalarParameterValue` "/Game/SnowBlowingLandscapeEffect/Materials/MPC_Preset_2.MPC_Preset_2" "Phase 2 Uvs Noise2" (`self.Phase 2 Uvs Noise2`))
  (`KismetMaterialLibrary.SetScalarParameterValue` "/Game/SnowBlowingLandscapeEffect/Materials/MPC_Preset_2.MPC_Preset_2" "Phase 2 X NoiseSpeed2" (`self.Phase 2 X NoiseSpeed2`))
  (`KismetMaterialLibrary.SetScalarParameterValue` "/Game/SnowBlowingLandscapeEffect/Materials/MPC_Preset_2.MPC_Preset_2" "Phase 2 Y NoiseSpeed2" (`self.Phase 2 Y NoiseSpeed2`))
  (`KismetMaterialLibrary.SetScalarParameterValue` "/Game/SnowBlowingLandscapeEffect/Materials/MPC_Preset_2.MPC_Preset_2" "Phase 2 Time2" (`self.Phase 2 Time2`))
  (`KismetMaterialLibrary.SetScalarParameterValue` "/Game/SnowBlowingLandscapeEffect/Materials/MPC_Preset_2.MPC_Preset_2" "Phase 2 Contrast2" (`self.Phase 2 Contrast2`))
  (`KismetMaterialLibrary.SetScalarParameterValue` "/Game/SnowBlowingLandscapeEffect/Materials/MPC_Preset_2.MPC_Preset_2" "Phase 2 Opacity2" (`self.Phase 2 Opacity2`))
  (`KismetMaterialLibrary.SetScalarParameterValue` "/Game/SnowBlowingLandscapeEffect/Materials/MPC_Preset_2.MPC_Preset_2" "Phase 1 DistortionStart2" (`self.Phase 1 DistortionStartRange2`))
  (`KismetMaterialLibrary.SetScalarParameterValue` "/Game/SnowBlowingLandscapeEffect/Materials/MPC_Preset_2.MPC_Preset_2" "Phase 1 DistortionEnd2" (`self.Phase 1 DistortionEndRange2`))
  (`KismetMaterialLibrary.SetVectorParameterValue` "/Game/SnowBlowingLandscapeEffect/Materials/MPC_Preset_2.MPC_Preset_2" "SnowColor2" (`self.SnowColor2`)))

(fn `UserConstructionScript`
  (`DecalComponent.SetDecalMaterial` (`self.SnowDecal`) (`self.Preset Selection`))
  (`SceneComponent.SetWorldScale3D` (`self.SnowDecal`) (`self.BoxEffectSize`))
  (`self.Preset1`)
  (`self.Preset2`)
  (`self.Preset 3`)
  (`self.Preset 4`)
  (`self.Preset 5`)
  (`self.Preset 6`))